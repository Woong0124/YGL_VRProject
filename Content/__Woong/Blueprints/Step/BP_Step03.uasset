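; BP_Step03 is a guided step that shows timed text on a player-attached UMG_Step widget, bracketed by BP_FirePawn egress and access events.
; Tick-driven Gates and DoOnces advance Intro lines, then spawn a BP_Select02 choice.
; False shows FalseSelect text; True plays TrueSelect lines before a timer destroys both actors.
; On destruction it spawns BP_Notice01 and BP_Notice02 at two points.
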(event Custom|E_Destroy
  (Default|CallEDDestroy (Variables|Default|GetSelect02))
  (Actor|DestroyActor))

(event Custom|ED_False
  (Variables|/Game/__Woong/Blueprints/Step/UMG_Step.UMG_Step_C|SetTextValue (Variables|Default|GetLocalUMG) (Variables|Default|GetFalseSelect)))

(event Custom|ED_True
  (Utilities|FlowControl|Gate true) ; enters at Open
)

(event EventBeginPlay
  (bind _asbp_fire_pawn (Utilities|Casting|CastToBP_FirePawn (Game|Player|GetPlayerPawn 0)))
  (Default|EDPawnEgressEvent _asbp_fire_pawn))

(event EventDestroyed
  (bind _asbp_fire_pawn (Utilities|Casting|CastToBP_FirePawn (Game|Player|GetPlayerPawn 0)))
  (Default|EDPawnAccessEvent _asbp_fire_pawn)
  (Game|SpawnActorfromClass "/Game/__Woong/Blueprints/Step/BP_Notice01.BP_Notice01_C" (Transformation|GetWorldTransform (Variables|Default|GetPoint1)) "Undefined" (Game|Player|GetPlayerPawn 0) 0)
  (Game|SpawnActorfromClass "/Game/__Woong/Blueprints/Step/BP_Notice02.BP_Notice02_C" (Transformation|GetWorldTransform (Variables|Default|GetPoint2)) "Undefined" (Game|Player|GetPlayerPawn 0) 0))

(event EventTick
  (params (DeltaSeconds :type Float%20%28single-precision%29))
  (bind _returnvalue (Transformation|GetActorLocation))
  (bind _returnvalue_2 (Transformation|GetActorRotation))
  (Utilities|FlowControl|Sequence
    (:then_0
      (Utilities|FlowControl|DoOnce false
        (:Completed
          (Transformation|AttachActorToActor (Game|Player|GetPlayerPawn 0) "None" "SnapToTarget" "SnapToTarget" "KeepRelative" true)
          (Transformation|SetRelativeLocationAndRotation (Variables|Default|GetWidget) "200.000000,0.000000,-55.000000" "170.000000,0.000000,180.000000" false false)
          (bind _asumg_step (Utilities|Casting|CastToUMG_Step (UserInterface|GetUserWidgetObject (Variables|Default|GetWidget))))
          (Variables|Default|SetLocalUMG _asumg_step))))
    (:then_1
      (Utilities|FlowControl|Gate false :!label _label
        (:Exit
          (Variables|/Game/__Woong/Blueprints/Step/UMG_Step.UMG_Step_C|SetTextValue (Variables|Default|GetLocalUMG) (Utilities|Array|Get(acopy) (Variables|Default|GetIntro) (Variables|Default|GetIndex)))
          (Utilities|FlowControl|Delay 2.8)
          (Math|Integer|IncrementInt (Variables|Default|GetIndex)))))
    (:then_2
      (if (== (Utilities|Array|LastIndex (Variables|Default|GetIntro)) (Variables|Default|GetIndex))
        (Utilities|FlowControl|DoOnce false
          (:Completed
            (Variables|Default|SetIndex 0)
            (bind _returnvalue_3 (Game|SpawnActorfromClass "/Game/__Woong/Blueprints/Step/BP_Select02.BP_Select02_C" (Math|Transform|MakeTransform (Math|Vector|MakeVector (+ (.x _returnvalue) 2e+02) (.y _returnvalue) (+ (.z _returnvalue) 6e+01)) (Math|Rotator|MakeRotator (.roll _returnvalue_2) (.pitch _returnvalue_2) (+ (.yaw _returnvalue_2) 1.8e+02))) "Undefined" self 0))
            (Variables|Default|SetSelect02 _returnvalue_3)
            (EventDispatchers|BindEventtoEDFalse (Variables|Default|GetSelect02) (delegate Custom|ED_False))
            (EventDispatchers|BindEventtoEDTrue (Variables|Default|GetSelect02) (delegate Custom|ED_True))
            (Utilities|FlowControl|Sequence
              (:then_0
                (goto _label Close))
              (:then_1
                (goto _label_3 Open)))))))
    (:then_3
      (Utilities|FlowControl|Gate true :!label _label_2
        (:Exit
          (Variables|/Game/__Woong/Blueprints/Step/UMG_Step.UMG_Step_C|SetTextValue (Variables|Default|GetLocalUMG) (Utilities|Array|Get(acopy) (Variables|Default|GetTrueSelect) (Variables|Default|GetIndex02)))
          (Utilities|FlowControl|Delay 2.8)
          (Math|Integer|IncrementInt (Variables|Default|GetIndex02)))))
    (:then_4
      (Utilities|FlowControl|Gate true :!label _label_3
        (:Exit
          (if (== (Utilities|Array|LastIndex (Variables|Default|GetTrueSelect)) (Variables|Default|GetIndex02))
            (Utilities|FlowControl|DoOnce false
              (:Completed
                (Variables|Default|SetIndex02 0)
                (Utilities|Time|SetTimerbyEvent (delegate Custom|E_Destroy) 3.5)
                (goto _label_2 Close)))))))))

(fn ConstructionScript)