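; BP_Select02 is a step actor showing a UMG_Select02 choice widget, operated through BP_FirePawn's left and right widget interaction components.
; BeginPlay fills the widget's two text values and enables input, so each trigger acts as a left-mouse click.
; Tick polls the widget's answer, firing EDTrue or EDFalse every frame while checked.
; A true answer also disables input once and binds EDDestroy to destroy the actor.
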(event Custom|ED_DestroyEvent
  (Actor|DestroyActor))

(event EventBeginPlay
  (Utilities|FlowControl|Sequence
    (:then_0
      (Input|EnableInput (Game|GetPlayerController 0))
      (bind _asbp_fire_pawn (Utilities|Casting|CastToBP_FirePawn (Game|Player|GetPlayerPawn 0)))
      (Variables|Default|SetWidget%20Interaction%20Left (Variables|/Game/__Woong/Blueprints/Pawn/BP_FirePawn.BP_FirePawn_C|GetWidgetInteractionLeft _asbp_fire_pawn))
      (Variables|Default|SetWidget%20Interaction%20Right (Variables|/Game/__Woong/Blueprints/Pawn/BP_FirePawn.BP_FirePawn_C|GetWidgetInteractionRight _asbp_fire_pawn)))
    (:then_1
      (bind _asumg_select_02 (Utilities|Casting|CastToUMG_Select02 (UserInterface|GetUserWidgetObject (Variables|Default|GetWidget))))
      (Variables|Default|SetAs%20UMG%20Select%2002 _asumg_select_02)
      (Variables|/Game/__Woong/Blueprints/Step/UMG_Select02.UMG_Select02_C|SetTextValue01 (Variables|Default|GetAs%20UMG%20Select%2002) (Variables|Default|GetValue01))
      (Variables|/Game/__Woong/Blueprints/Step/UMG_Select02.UMG_Select02_C|SetTextValue02 (Variables|Default|GetAs%20UMG%20Select%2002) (Variables|Default|GetValue02)))))

(event EventTick
  (params (DeltaSeconds :type Float%20%28single-precision%29))
  (if (Variables|/Game/__Woong/Blueprints/Step/UMG_Select02.UMG_Select02_C|GetIsCheck (Variables|Default|GetAs%20UMG%20Select%2002))
    (if (Variables|/Game/__Woong/Blueprints/Step/UMG_Select02.UMG_Select02_C|GetIsTrue (Variables|Default|GetAs%20UMG%20Select%2002))
      (Default|CallEDTrue)
      (Utilities|FlowControl|DoOnce false
        (:Completed
          (Input|DisableInput (Game|GetPlayerController 0))
          (EventDispatchers|BindEventtoEDDestroy (delegate Custom|ED_DestroyEvent))))
      (else
        (Default|CallEDFalse)))))

(event Input|ActionEvents|InputActionTriggerLeft
  (params (Key :type Key%20Structure :default "None"))
  (bind _widget_interaction_left (Variables|Default|GetWidget%20Interaction%20Left))
  (:Pressed
    (Class|WidgetInteractionComponent|PressPointerKey _widget_interaction_left "LeftMouseButton"))
  (:Released
    (Class|WidgetInteractionComponent|ReleasePointerKey _widget_interaction_left "LeftMouseButton")))

(event Input|ActionEvents|InputActionTriggerRight
  (params (Key :type Key%20Structure :default "None"))
  (bind _widget_interaction_right (Variables|Default|GetWidget%20Interaction%20Right))
  (:Pressed
    (Class|WidgetInteractionComponent|PressPointerKey _widget_interaction_right "LeftMouseButton"))
  (:Released
    (Class|WidgetInteractionComponent|ReleasePointerKey _widget_interaction_right "LeftMouseButton")))

(fn ConstructionScript)