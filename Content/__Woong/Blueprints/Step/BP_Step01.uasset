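; BP_Step01 is a sequence step that shows intro text on a widget attached to the player pawn, then hands off to BP_Step02.
; BeginPlay triggers the fire pawn's egress event; Tick attaches the actor once and pushes Intro lines to UMG_Step through a gate, using a Delay to pace the index.
; At the last index it closes the gate, fades the camera and self-destroys on a timer.
; Destroyed spawns the next step at NextPoint.
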(event Custom|E_Destroy
  (Actor|DestroyActor))

(event EventBeginPlay
  (bind _asbp_fire_pawn (Utilities|Casting|CastToBP_FirePawn (Game|Player|GetPlayerPawn 0)))
  (Default|EDPawnEgressEvent _asbp_fire_pawn))

(event EventDestroyed
  (Game|SpawnActorfromClass "/Game/__Woong/Blueprints/Step/BP_Step02.BP_Step02_C" (Math|Transform|MakeTransform (Transformation|GetWorldLocation (Variables|Default|GetNextPoint))) "Undefined" (Game|Player|GetPlayerPawn 0) 0))

(event EventTick
  (params (DeltaSeconds :type Float%20%28single-precision%29))
  (Utilities|FlowControl|Sequence
    (:then_0
      (Utilities|FlowControl|DoOnce false
        (:Completed
          (Transformation|AttachActorToActor (Game|Player|GetPlayerPawn 0) "None" "SnapToTarget" "SnapToTarget" "KeepRelative" true)
          (Transformation|SetRelativeLocationAndRotation (Variables|Default|GetWidget) "200.000000,0.000000,-55.000000" "170.000000,0.000000,180.000000" false false)
          (bind _asumg_step (Utilities|Casting|CastToUMG_Step (UserInterface|GetUserWidgetObject (Variables|Default|GetWidget))))
          (Variables|Default|SetLocalUMG _asumg_step))))
    (:then_1
      (Utilities|FlowControl|Gate false :!label _label
        (:Exit
          (Variables|/Game/__Woong/Blueprints/Step/UMG_Step.UMG_Step_C|SetTextValue (Variables|Default|GetLocalUMG) (Utilities|Array|Get(acopy) (Variables|Default|GetIntro) (Variables|Default|GetIndex)))
          (Utilities|FlowControl|Delay 2.8)
          (Math|Integer|IncrementInt (Variables|Default|GetIndex)))))
    (:then_2
      (if (== (Utilities|Array|LastIndex (Variables|Default|GetIntro)) (Variables|Default|GetIndex))
        (Utilities|FlowControl|DoOnce false
          (:Completed
            (Utilities|FlowControl|Sequence
              (:then_0
                (goto _label Close))
              (:then_1
                (Utilities|Time|SetTimerbyEvent (delegate Custom|E_Destroy) 5.0)
                (Utilities|FlowControl|Delay 2.5)
                (CameraFades|StartCameraFade :self (Game|GetPlayerCameraManager 0) :ToAlpha 1.0 :Duration 2.0 :bHoldWhenFinished true)))))))))

(fn ConstructionScript)