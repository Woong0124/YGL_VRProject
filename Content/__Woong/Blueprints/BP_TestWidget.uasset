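; BP_TestWidget is a test Blueprint that turns VR trigger input into left mouse clicks on widgets.
; TriggerLeft and TriggerRight press and release the pointer key on their respective Widget Interaction component references.
; The setup that enables input and fetches those references from BP_RealVRPawn is disconnected from the empty BeginPlay, so it never runs and nothing here assigns them.
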(event EventBeginPlay)

(event Input|ActionEvents|InputActionTriggerLeft
  (params (Key :type Key%20Structure :default "None"))
  (bind _widgetinteractionrefleft (Variables|Default|GetWidgetInteractionRefLeft))
  (:Pressed
    (Class|WidgetInteractionComponent|PressPointerKey _widgetinteractionrefleft "LeftMouseButton"))
  (:Released
    (Class|WidgetInteractionComponent|ReleasePointerKey _widgetinteractionrefleft "LeftMouseButton")))

(event Input|ActionEvents|InputActionTriggerRight
  (params (Key :type Key%20Structure :default "None"))
  (bind _widgetinteractionrefright (Variables|Default|GetWidgetInteractionRefRight))
  (:Pressed
    (Class|WidgetInteractionComponent|PressPointerKey _widgetinteractionrefright "LeftMouseButton"))
  (:Released
    (Class|WidgetInteractionComponent|ReleasePointerKey _widgetinteractionrefright "LeftMouseButton")))

(fn ConstructionScript)